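; GenericFunctions is a set of generic math helpers that add to a float and negate floats or integers.
; Each helper computes a new value and passes it with the variable reference to ManipulateFloatInternal or ManipulateIntInternal, returning that call's result.
; The FloatRef and IntegerRef inputs suggest in-place modification, though the internal helpers are not defined here.
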(fn AddFloat
  (params (Var :type Float%20%28double-precision%29%20%28by%20ref%29) (Value :type Float%20%28double-precision%29))
  (bind _result (Utilities|ManipulateFloatInternal Var (+ Var Value))
    (:%20%20
      (return _result))))

(fn InvertFloat
  (params (Var :type Float%20%28double-precision%29%20%28by%20ref%29))
  (bind _result (Utilities|ManipulateFloatInternal Var (* Var -1.0))
    (:%20%20
      (return _result))))

(fn InvertInt
  (params (Var :type Integer%20%28by%20ref%29))
  (bind _result (Utilities|ManipulateIntInternal Var (* Var -1))
    (:%20%20
      (return _result))))