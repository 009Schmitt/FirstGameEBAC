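; Player-management Blueprint that exposes getters and setters for the third-person character's life, coins and invincibility, plus HUD and input-mode helpers.
; Each call casts player 0's character and accesses its Stats struct or HUD widget, with coin and life changes pushed to the HUD.
; Life is clamped, and damage turns invincibility on while healing turns it off; SetLife itself never checks that flag.
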(fn GetCoins
  (bind _player (CallFunction|GetPlayer))
  (return (.coin (Variables|/Game/ThirdPerson/Blueprints/BP_ThirdPersonCharacter.BP_ThirdPersonCharacter_C|GetStats _player))))

(fn SetCoins
  (params (Add :type Boolean) (Quantity :type Integer))
  (bind _player (CallFunction|GetPlayer))
  (if Add
    (Variables|/Game/ThirdPerson/Blueprints/BP_ThirdPersonCharacter.BP_ThirdPersonCharacter_C|SetStats _player (Utilities|Struct|MakePlayerStats (.life (Variables|/Game/ThirdPerson/Blueprints/BP_ThirdPersonCharacter.BP_ThirdPersonCharacter_C|GetStats _player)) (+ Quantity (.coin (Variables|/Game/ThirdPerson/Blueprints/BP_ThirdPersonCharacter.BP_ThirdPersonCharacter_C|GetStats _player))) (.invensiblemode (Variables|/Game/ThirdPerson/Blueprints/BP_ThirdPersonCharacter.BP_ThirdPersonCharacter_C|GetStats _player))))
    (else
      (Variables|/Game/ThirdPerson/Blueprints/BP_ThirdPersonCharacter.BP_ThirdPersonCharacter_C|SetStats _player (Utilities|Struct|MakePlayerStats (.life (Variables|/Game/ThirdPerson/Blueprints/BP_ThirdPersonCharacter.BP_ThirdPersonCharacter_C|GetStats _player)) (- (.coin (Variables|/Game/ThirdPerson/Blueprints/BP_ThirdPersonCharacter.BP_ThirdPersonCharacter_C|GetStats _player)) Quantity) (.invensiblemode (Variables|/Game/ThirdPerson/Blueprints/BP_ThirdPersonCharacter.BP_ThirdPersonCharacter_C|GetStats _player))))))
  (bind _coins (CallFunction|GetCoins))
  (bind _hud (CallFunction|GetPlayerHUD))
  (Default|ChangeCoin _hud _coins))

(fn GetPlayer
  (bind _asbp_third_person_character (Utilities|Casting|CastToBP_ThirdPersonCharacter (Game|GetPlayerCharacter 0)))
  (return _asbp_third_person_character))

(fn GetLife
  (bind _player (CallFunction|GetPlayer))
  (return (.life (Variables|/Game/ThirdPerson/Blueprints/BP_ThirdPersonCharacter.BP_ThirdPersonCharacter_C|GetStats _player))))

(fn SetLife
  (params (Add :type Boolean) (Quantity :type Float%20%28double-precision%29))
  (bind _player (CallFunction|GetPlayer))
  (if Add
    (Variables|/Game/ThirdPerson/Blueprints/BP_ThirdPersonCharacter.BP_ThirdPersonCharacter_C|SetStats _player (Utilities|Struct|MakePlayerStats (Math|Float|Clamp(Float) (+ (.life (Variables|/Game/ThirdPerson/Blueprints/BP_ThirdPersonCharacter.BP_ThirdPersonCharacter_C|GetStats _player)) Quantity) 0.0 1e+02) (.coin (Variables|/Game/ThirdPerson/Blueprints/BP_ThirdPersonCharacter.BP_ThirdPersonCharacter_C|GetStats _player)) false))
    (else
      (Variables|/Game/ThirdPerson/Blueprints/BP_ThirdPersonCharacter.BP_ThirdPersonCharacter_C|SetStats _player (Utilities|Struct|MakePlayerStats (Math|Float|Clamp(Float) (- (.life (Variables|/Game/ThirdPerson/Blueprints/BP_ThirdPersonCharacter.BP_ThirdPersonCharacter_C|GetStats _player)) Quantity) 0.0 1e+02) (.coin (Variables|/Game/ThirdPerson/Blueprints/BP_ThirdPersonCharacter.BP_ThirdPersonCharacter_C|GetStats _player)) true))))
  (bind _life (CallFunction|GetLife))
  (bind _hud (CallFunction|GetPlayerHUD))
  (Default|ChangeLifeBar _hud _life))

(fn GetInvencibility
  (bind _player (CallFunction|GetPlayer))
  (return (.invensiblemode (Variables|/Game/ThirdPerson/Blueprints/BP_ThirdPersonCharacter.BP_ThirdPersonCharacter_C|GetStats _player))))

(fn SetInvencibility
  (params (Invencibility :type Boolean))
  (bind _player (CallFunction|GetPlayer))
  (Variables|/Game/ThirdPerson/Blueprints/BP_ThirdPersonCharacter.BP_ThirdPersonCharacter_C|SetStats _player (Utilities|Struct|MakePlayerStats (.life (Variables|/Game/ThirdPerson/Blueprints/BP_ThirdPersonCharacter.BP_ThirdPersonCharacter_C|GetStats _player)) (.coin (Variables|/Game/ThirdPerson/Blueprints/BP_ThirdPersonCharacter.BP_ThirdPersonCharacter_C|GetStats _player)) Invencibility)))

(fn GetPlayerHUD
  (bind _player (CallFunction|GetPlayer))
  (return (Variables|/Game/ThirdPerson/Blueprints/BP_ThirdPersonCharacter.BP_ThirdPersonCharacter_C|GetHUD _player)))

(fn ClearHUD
  (bind _player (CallFunction|GetPlayer))
  (Widget|RemovefromParent (Variables|/Game/ThirdPerson/Blueprints/BP_ThirdPersonCharacter.BP_ThirdPersonCharacter_C|GetHUD _player)))

(fn SetPlayerInput
  (params (IsGameOnly? :type Boolean))
  (bind _returnvalue (Game|GetPlayerController 0))
  (if IsGameOnly?
    (Input|SetInputModeGameOnly _returnvalue false)
    (Variables|/Script/Engine.PlayerController|SetbShowMouseCursor _returnvalue false)
    (else
      (Input|SetInputModeUIOnly _returnvalue 0 "DoNotLock" false)
      (Variables|/Script/Engine.PlayerController|SetbShowMouseCursor _returnvalue true))))