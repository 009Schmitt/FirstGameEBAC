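; Collectible coin that bobs and spins in the level until an actor overlaps it.
; On overlap it calls PickUp, adds CoinValue through SetCoins and destroys itself, with no check on which actor touched it.
; From BeginPlay, a looping Delay stands in for Tick, offsetting the mesh's height by the Oscilation curve, wrapped at its end time, and advancing its yaw by a fixed step.
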(event EventBeginPlay
  (bind _oscilation (Variables|Default|GetOscilation))
  (Variables|Default|SetStart%20Position (Variables|/Script/Engine.SceneComponent|GetRelativeLocation (Variables|Default|GetStaticMesh)))
  (Variables|Default|SetOscilation%20Max (.MaxTime (Math|Curves|GetTimeRange _oscilation)))
  (Transformation|SetRelativeLocation (Variables|Default|GetStaticMesh) (Math|Vector|MakeVector (.x (Variables|Default|GetStart%20Position)) (.y (Variables|Default|GetStart%20Position)) (+ (.z (Variables|Default|GetStart%20Position)) (Math|Curves|GetFloatValue _oscilation (Variables|Default|GetIn%20Time%20Oscilation)))) false false :!label _label)
  (Transformation|SetRelativeRotation (Variables|Default|GetStaticMesh) (Math|Rotator|MakeRotator 9e+01 0.0 (Variables|Default|GetRotation)) false false)
  (bind _result (CallFunction|AddFloat (Variables|Default|GetIn%20Time%20Oscilation) 0.1))
  (if (>= _result (Variables|Default|GetOscilation%20Max))
    (Variables|Default|SetIn%20Time%20Oscilation 0.0))
  (CallFunction|AddFloat (Variables|Default|GetRotation) (Variables|Default|GetInTimeRotation))
  (Utilities|FlowControl|Delay 0.02)
  (goto _label))

(event Collision|EventActorBeginOverlap
  (params (OtherActor :type Actor%20Object%20Reference))
  (CallFunction|PickUp)
  (CallFunction|SetCoins true (Variables|Default|GetCoinValue))
  (Actor|DestroyActor))

(fn ConstructionScript
  (|CallParentFunction))