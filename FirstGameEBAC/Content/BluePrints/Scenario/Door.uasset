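; Coin-gated door that swings open when an actor overlaps it and the coin count is at least ten.
; On success it deducts the coins and destroys the Box component, otherwise it prints a message asking for more gold.
; The swing is a Delay-based loop in the event graph that yaws the static mesh in one-degree steps through roughly a quarter turn, tracked by a counter.
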(event Collision|EventActorBeginOverlap
  (params (OtherActor :type Actor%20Object%20Reference))
  (bind _coins (CallFunction|GetCoins))
  (if (>= _coins 10)
    (Development|PrintString "Thanks for the MONEY !!!" true true "(R=0.687500,G=0.682946,B=0.082720,A=1.000000)" 5.0)
    (Components|DestroyComponent (Variables|Default|GetBox))
    (CallFunction|SetCoins false 10)
    (Transformation|AddWorldRotation (Variables|Default|GetStaticMesh) (Math|Rotator|MakeRotator 0.0 0.0 -1.0) false false :!label _label)
    (bind _result (Math|Integer|IncrementInt (Variables|Default|GetCounter))
      (:%20%20
        (if (<= _result 90)
          (Utilities|FlowControl|Delay 0.02)
          (goto _label))))
    (else
      (Development|PrintString "NEED MORE GOLD!!!!!" true true "(R=0.245833,G=0.000000,B=0.004710,A=1.000000)" 5.0))))

(fn ConstructionScript)