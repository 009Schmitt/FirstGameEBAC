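; EndStage is a stage-finish trigger actor that sinks a mesh and then shows the winner screen.
; Any actor overlap starts a Delay-driven loop that lowers StaticMesh1 in small relative Z steps until it passes a fixed depth.
; It then switches the player HUD to WinnerScreen and disables player input.
; The overlap has no actor filter or guard against retriggering.
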(event Collision|EventActorBeginOverlap
  (params (OtherActor :type Actor%20Object%20Reference))
  (bind _staticmesh1 (Variables|Default|GetStaticMesh1))
  (bind _relativelocation (Variables|/Script/Engine.SceneComponent|GetRelativeLocation _staticmesh1))
  (bind _output_get (Variables|Default|SetPosition (.z _relativelocation)))
  (Transformation|SetRelativeLocation _staticmesh1 (Math|Vector|MakeVector (.x _relativelocation) (.y _relativelocation) _output_get) false false :!label _label)
  (bind _result (CallFunction|AddFloat (Variables|Default|GetPosition) -3.0))
  (if (>= _result -6e+01)
    (Utilities|FlowControl|Delay 0.02)
    (goto _label)
    (else
      (bind _hud (CallFunction|GetPlayerHUD))
      (CallFunction|ChangeScreen _hud "/Game/HUD/WinnerScreen.WinnerScreen_C")
      (CallFunction|SetPlayerInput false))))

(fn ConstructionScript)