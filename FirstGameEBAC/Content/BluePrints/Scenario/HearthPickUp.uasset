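; Heart pickup actor that adds life on overlap with any actor, then destroys itself.
; Overlap calls PickUp and SetLife in add mode with LifeAmount, with no filter on the overlapping actor.
; From BeginPlay, a self-looping Delay chain animates the mesh instead of Tick, bobbing it along the Oscilation float curve and spinning its yaw.
; Curve time advances in fixed steps and wraps at the curve's end.
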(event EventBeginPlay
  (bind _oscilation (Variables|Default|GetOscilation))
  (Variables|Default|SetStartPosition (Variables|/Script/Engine.SceneComponent|GetRelativeLocation (Variables|Default|GetStaticMesh)))
  (Variables|Default|SetOscilationMax (.MaxTime (Math|Curves|GetTimeRange _oscilation)))
  (Transformation|SetRelativeLocation (Variables|Default|GetStaticMesh) (Math|Vector|MakeVector (.x (Variables|Default|GetStartPosition)) (.y (Variables|Default|GetStartPosition)) (+ (.z (Variables|Default|GetStartPosition)) (Math|Curves|GetFloatValue _oscilation (Variables|Default|GetInTimeOscilation)))) false false :!label _label)
  (Transformation|SetRelativeRotation (Variables|Default|GetStaticMesh) (Math|Rotator|MakeRotator 0.0 0.0 (Variables|Default|GetRotation)) false false)
  (bind _result (CallFunction|AddFloat (Variables|Default|GetInTimeOscilation) 0.05))
  (if (>= _result (Variables|Default|GetOscilationMax))
    (Variables|Default|SetInTimeOscilation 0.0))
  (CallFunction|AddFloat (Variables|Default|GetRotation) (Variables|Default|GetInTimeRotation))
  (Utilities|FlowControl|Delay 0.02)
  (goto _label))

(event Collision|EventActorBeginOverlap
  (params (OtherActor :type Actor%20Object%20Reference))
  (CallFunction|PickUp)
  (CallFunction|SetLife true (Variables|Default|GetLifeAmount))
  (Actor|DestroyActor))

(fn ConstructionScript
  (|CallParentFunction))