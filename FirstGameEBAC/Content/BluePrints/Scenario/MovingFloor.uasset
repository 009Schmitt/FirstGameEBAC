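; A moving floor Blueprint that slides its static mesh back and forth indefinitely.
; A self-repeating loop started on BeginPlay applies a local offset of Direction times Speed after each short delay.
; Each pass also advances an elapsed counter by a fixed step, flipping Direction and resetting the counter once it exceeds Duration.
; Movement is stepped per loop pass rather than scaled by delta time.
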(event EventBeginPlay
  (Transformation|AddLocalOffset (Variables|Default|GetStaticMesh) (Math|Vector|MakeVector (* (Variables|Default|GetDirection) (Variables|Default|GetSpeed)) 0.0 0.0) false false :!label _label)
  (bind _result (CallFunction|AddFloat (Variables|Default|GetActualDuration) 0.05))
  (if (<= _result (Variables|Default|GetDuration))
    _
    (else
      (CallFunction|InvertInt (Variables|Default|GetDirection))
      (Variables|Default|SetActualDuration 0.0)))
  (Utilities|FlowControl|Delay 0.02)
  (goto _label))

(fn ConstructionScript)